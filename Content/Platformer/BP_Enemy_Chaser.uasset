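; Platformer chaser enemy that pursues the player, rams them and can be killed by landing on its head.
; While the player overlaps DetectionZone, Tick turns it toward them using X/Y only and adds movement input straight at them, without pathfinding.
; HitZone overlaps launch the player and cost one Health, destroying it with fire and explosion sound at zero.
; Capsule hits knock the player back along the enemy's velocity and deal damage.
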(event OnComponentBeginOverlap(DetectionZone)
  (params (OverlappedComponent :type Primitive%20Component%20Object%20Reference) (OtherActor :type Actor%20Object%20Reference) (OtherComp :type Primitive%20Component%20Object%20Reference) (OtherBodyIndex :type Integer) (bFromSweep :type Boolean) (SweepResult :type Hit%20Result%20Structure%20%28by%20ref%29))
  ;[1 0.8729 0.4688] Check If Detecting Player
  (if (== OtherActor (Variables|Default|GetPlayerReference))
    (Variables|Default|SetCanDetectPlayer true)))

(event OnComponentEndOverlap(DetectionZone)
  (params (OverlappedComponent :type Primitive%20Component%20Object%20Reference) (OtherActor :type Actor%20Object%20Reference) (OtherComp :type Primitive%20Component%20Object%20Reference) (OtherBodyIndex :type Integer))
  ;[1 0.8729 0.4688] Check If Detecting Player
  (if (== OtherActor (Variables|Default|GetPlayerReference))
    (Variables|Default|SetCanDetectPlayer false)))

(event OnComponentBeginOverlap(HitZone)
  (params (OverlappedComponent :type Primitive%20Component%20Object%20Reference) (OtherActor :type Actor%20Object%20Reference) (OtherComp :type Primitive%20Component%20Object%20Reference) (OtherBodyIndex :type Integer) (bFromSweep :type Boolean) (SweepResult :type Hit%20Result%20Structure%20%28by%20ref%29))
  (bind _enemy_reference (Variables|Default|GetEnemy%20Reference))
  (bind _returnvalue (Transformation|GetActorLocation _enemy_reference))
  ;[0.08476 0.2573 1] Land On  Head
  (if (== OtherActor (Variables|Default|GetPlayerReference))
    (Utilities|FlowControl|Sequence
      (:then_0
        ;[0.01995 1 0.9602] Launch Character
        (Character|LaunchCharacter (Variables|Default|GetPlayerReference) (Variables|Default|GetLaunch%20Direction) false false))
      (:then_1
        ;[1 0.9781 0.0603] Calculate And Lower Enemy Health
        (Variables|Default|SetHealth (- (Variables|Default|GetHealth) 1))
        ;[0 0.2135 0.007358] Destroy Enemy
        (if (<= (Variables|Default|GetHealth) 0)
          (Utilities|FlowControl|Sequence
            (:then_0
              ;[1 0.1823 0.1823] Explode When Destroyed
              (Effects|SpawnEmitteratLocation "/Game/StarterContent/Particles/P_Fire.P_Fire" _returnvalue)
              (Audio|SpawnSoundatLocation "/Game/StarterContent/Audio/Explosion01.Explosion01" _returnvalue "0, 0, 0" 1.0 1.0 0.0 0 0))
            (:then_1
              (Actor|DestroyActor))))))))

(event OnComponentHit(CapsuleComponent)
  (params (HitComponent :type Primitive%20Component%20Object%20Reference) (OtherActor :type Actor%20Object%20Reference) (OtherComp :type Primitive%20Component%20Object%20Reference) (NormalImpulse :type Vector :default "0, 0, 0") (Hit :type Hit%20Result%20Structure%20%28by%20ref%29))
  ;[1 1 1] Hit Knockback
  (if (== OtherActor (Variables|Default|GetPlayerReference))
    (Character|LaunchCharacter (Variables|Default|GetPlayerReference) (* (Transformation|GetVelocity) (Variables|Default|GetKnockBackStrength)) false false)
    ;[0.125 0.04769 0] Damage Player
    (Variables|/Game/Platformer/BP_ThirdPersonCharacter.BP_ThirdPersonCharacter_C|SetHealth (Variables|Default|GetPlayerReference) (- (Variables|/Game/Platformer/BP_ThirdPersonCharacter.BP_ThirdPersonCharacter_C|GetHealth (Variables|Default|GetPlayerReference)) (Variables|Default|GetDamage)))))

(event EventBeginPlay
  ;[1 0.4792 0.7873] Get Player Reference
  (bind _asbp_third_person_character (Utilities|Casting|CastToBP_ThirdPersonCharacter (Game|Player|GetPlayerPawn 0)))
  (Variables|Default|SetPlayerReference _asbp_third_person_character))

(event EventTick
  (params (DeltaSeconds :type Float%20%28single-precision%29))
  (bind _returnvalue (Transformation|GetActorLocation))
  (bind _playerreference (Variables|Default|GetPlayerReference))
  (bind _returnvalue_2 (Transformation|GetActorLocation _playerreference))
  ;[0.2292 0.04855 0.07141] If Detected
  (if (Variables|Default|GetCanDetectPlayer)
    (Utilities|FlowControl|Sequence
      (:then_0
        ;[0.2457 0.349 0.209] Look At Player
        (Transformation|SetActorRotation (Math|Rotator|FindLookatRotation (Math|Vector|MakeVector (.x _returnvalue) (.y _returnvalue) 0.0) (Math|Vector|MakeVector (.x _returnvalue_2) (.y _returnvalue_2) 0.0))))
      (:then_1
        ;[0.4219 1 0.8464] Chase Player
        (Pawn|Input|AddMovementInput (Math|Vector|Normalize (- (Transformation|GetActorLocation (Variables|Default|GetPlayerReference)) (Transformation|GetActorLocation))) 1.0 false)))))

(fn ConstructionScript)