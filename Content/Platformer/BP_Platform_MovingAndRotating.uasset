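; BP_Platform_MovingAndRotating is a platform actor that moves back and forth while continuously spinning.
; On BeginPlay it enables movement and starts a looping timer that negates Direction every MovementDuration.
; Tick offsets the actor along normalized Direction by Speed, without sweep, and separately adds local rotation from SpinDirection and SpinSpeed.
; Both steps apply per frame without DeltaSeconds scaling, and CanPlatformMove gates only the translation.
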(event Custom|FlipDirection
  ;[1 0.2448 0.2448] Platform Flip Direction
  (Variables|Default|SetDirection (* (Variables|Default|GetDirection) -1.0)))

(event EventBeginPlay
  ;[1 0.2448 0.2448] Platform Flip Direction
  (|CallParentFunction)
  (Utilities|FlowControl|Sequence
    (:then_0
      (Variables|Default|SetCanPlatformMove true))
    (:then_1
      (Utilities|Time|SetTimerbyEvent (delegate Custom|FlipDirection) (Variables|Default|GetMovementDuration) true))))

(event EventTick
  (params (DeltaSeconds :type Float%20%28single-precision%29))
  ;[0.5038 0.5785 1] Platform Movement
  (|CallParentFunction DeltaSeconds)
  (Utilities|FlowControl|Sequence
    (:then_0
      (if (Variables|Default|GetCanPlatformMove)
        (Transformation|AddActorWorldOffset (* (Math|Vector|Normalize (Variables|Default|GetDirection)) (Variables|Default|GetSpeed)))))
    (:then_1
      ;[1 0.2746 0.5289] Rotation
      (Transformation|AddActorLocalRotation (* (Variables|Default|GetSpinDirection) (Variables|Default|GetSpinSpeed)) false false))))

(fn ConstructionScript
  (|CallParentFunction))