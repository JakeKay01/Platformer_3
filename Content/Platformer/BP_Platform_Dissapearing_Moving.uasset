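; Platformer platform that moves while the player stands on it, then temporarily disappears after its lifetime runs out.
; A collision box tracks the player, letting Tick count standing time and offset the actor by Speed each frame, unscaled by delta time.
; A looping timer reverses Direction independently of the player.
; At the lifetime limit it hides and disables collision, then after a delay restores its starting transform, visibility and collision.
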(event OnComponentBeginOverlap(CollisionBox)
  (params (OverlappedComponent :type Primitive%20Component%20Object%20Reference) (OtherActor :type Actor%20Object%20Reference) (OtherComp :type Primitive%20Component%20Object%20Reference) (OtherBodyIndex :type Integer) (bFromSweep :type Boolean) (SweepResult :type Hit%20Result%20Structure%20%28by%20ref%29))
  ;[1 0.2753 0.09495] Collider Check
  (if (== OtherActor (Game|Player|GetPlayerPawn 0))
    (Utilities|FlowControl|Sequence
      (:then_0
        (Development|PrintString "Player is on Platform"))
      (:then_1
        (Variables|Default|SetIsPlayerOnPlatform true)))))

(event OnComponentEndOverlap(CollisionBox)
  (params (OverlappedComponent :type Primitive%20Component%20Object%20Reference) (OtherActor :type Actor%20Object%20Reference) (OtherComp :type Primitive%20Component%20Object%20Reference) (OtherBodyIndex :type Integer))
  ;[1 0.2753 0.09495] Collider Check
  (if (== OtherActor (Game|Player|GetPlayerPawn 0))
    (Utilities|FlowControl|Sequence
      (:then_0
        (Development|PrintString "Player is off Platform"))
      (:then_1
        (Variables|Default|SetIsPlayerOnPlatform false)))))

(event Custom|FlipDirection
  ;[1 0.2448 0.2448] Platform Flip Direction
  (Variables|Default|SetDirection (* (Variables|Default|GetDirection) -1.0)))

(event Custom|ReturnToStart
  ;[0 0.2886 1] Reset Platform To Default
  (Transformation|SetWorldTransform (Variables|Default|GetDefaultSceneRoot) (Math|Transform|MakeTransform (Variables|Default|GetStartLocation) (Variables|Default|GetStartRotation) (Variables|Default|GetStartScale)) false true)
  (Rendering|SetActorHiddenInGame false)
  (Collision|SetCollisionEnabled (Variables|Default|GetCube) "QueryAndPhysics")
  (Collision|SetCollisionEnabled (Variables|Default|GetCollision%20Box) "QueryAndPhysics"))

(event EventTick
  (params (DeltaSeconds :type Float%20%28single-precision%29))
  ;[0.7955 0.4314 1] Set Platform Timer
  (|CallParentFunction DeltaSeconds)
  (if (Variables|Default|GetIsPlayerOnPlatform)
    (bind _output_get (Variables|Default|SetTimeOnPlatform (+ (Variables|Default|GetTimeOnPlatform) DeltaSeconds)))
    (Utilities|FlowControl|Sequence
      (:then_0
        ;[0.1399 0.8398 1] Count to 5
        (if (>= (Variables|Default|GetTimeOnPlatform) (Variables|Default|GetPlatformLifetime))
          ;[0.4416 0.3083 1] Hide and Disable Platform
          (Rendering|SetActorHiddenInGame true)
          (Collision|SetCollisionEnabled (Variables|Default|GetCube) "NoCollision")
          (Collision|SetCollisionEnabled (Variables|Default|GetCollision%20Box) "NoCollision")
          (Utilities|FlowControl|Delay (Variables|Default|GetTimeInvisible))
          (CallFunction|ReturntoStart)))
      (:then_1
        (Development|PrintString (Utilities|String|ToString(Float) _output_get)))
      (:then_2
        ;[0.5038 0.5785 1] Platform Movement
        (if (Variables|Default|GetCanPlatformMove)
          (Transformation|AddActorWorldOffset (* (Math|Vector|Normalize (Variables|Default|GetDirection)) (Variables|Default|GetSpeed))))))
    (else
      (Variables|Default|SetTimeOnPlatform 0.0))))

(event EventBeginPlay
  (bind _returnvalue (Transformation|GetActorTransform))
  ;[1 0.2448 0.2448] Platform Flip Direction
  (|CallParentFunction)
  (Utilities|FlowControl|Sequence
    (:then_0
      (Variables|Default|SetCanPlatformMove true))
    (:then_1
      (Utilities|Time|SetTimerbyEvent (delegate Custom|FlipDirection) (Variables|Default|GetMovementDuration) true))
    (:then_2
      ;[1 0.8538 0.5277] Set Start Variables
      (Variables|Default|SetStartLocation (.location _returnvalue))
      (Variables|Default|SetStartRotation (.rotation _returnvalue))
      (Variables|Default|SetStartScale (.scale _returnvalue)))))

(fn ConstructionScript
  (|CallParentFunction))